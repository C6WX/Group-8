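; BP_Teller1 is an interactable teller NPC in the first flashback that records how the player resolves the teller encounter.
; Interact starts dialogue 0 on its BPC dialogue component.
; DialogueEvent switches on the event name and adds a matching gameplay tag, such as killing, sparing, intervening or persuading Kylie, to the player character's owned tags.
; Only the Killed Teller branch performs the character cast whose result the other branches reuse.
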(event EventInteract
  (Default|StartDialog (Variables|Default|GetBPC_DialogueComponent)))

(event EventDialogueEvent
  (params (EventName :type Text))
  (switch string (Utilities|String|ToString(Text) EventName)
    (:KilledTeller
      (bind _asbp_third_person_character (Utilities|Casting|CastToBP_ThirdPersonCharacter (Game|GetPlayerCharacter 0)))
      (GameplayTags|AddGameplayTag (Variables|/Game/Dynamic/Blueprints/Core/MC/BP_ThirdPersonCharacter.BP_ThirdPersonCharacter_C|GetOwnedGameplayTags _asbp_third_person_character) "(TagName=\"KilledTeller\")" :!class /Script/GameplayTags.BlueprintGameplayTagLibrary))
    (:LeftTellerAlive
      (GameplayTags|AddGameplayTag (Variables|/Game/Dynamic/Blueprints/Core/MC/BP_ThirdPersonCharacter.BP_ThirdPersonCharacter_C|GetOwnedGameplayTags _asbp_third_person_character) "(TagName=\"LeftTellerAlive\")" :!class /Script/GameplayTags.BlueprintGameplayTagLibrary))
    (:LeftKylieToKillTeller
      (GameplayTags|AddGameplayTag (Variables|/Game/Dynamic/Blueprints/Core/MC/BP_ThirdPersonCharacter.BP_ThirdPersonCharacter_C|GetOwnedGameplayTags _asbp_third_person_character) "(TagName=\"LeftKylieToKillTeller\")" :!class /Script/GameplayTags.BlueprintGameplayTagLibrary))
    (:Intervened
      (GameplayTags|AddGameplayTag (Variables|/Game/Dynamic/Blueprints/Core/MC/BP_ThirdPersonCharacter.BP_ThirdPersonCharacter_C|GetOwnedGameplayTags _asbp_third_person_character) "(TagName=\"Intervened\")" :!class /Script/GameplayTags.BlueprintGameplayTagLibrary))
    (:PersuadeKylie
      (GameplayTags|AddGameplayTag (Variables|/Game/Dynamic/Blueprints/Core/MC/BP_ThirdPersonCharacter.BP_ThirdPersonCharacter_C|GetOwnedGameplayTags _asbp_third_person_character) "(TagName=\"PersuadedKylie\")" :!class /Script/GameplayTags.BlueprintGameplayTagLibrary))))

(fn ConstructionScript)