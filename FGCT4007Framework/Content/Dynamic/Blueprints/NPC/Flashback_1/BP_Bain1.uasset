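; BP_Bain1 is the Bain NPC for the first flashback, talked to through interaction.
; Interacting starts dialogue 0 on its BPC dialogue component, and the "Van Line Done" dialogue event removes the VanLineNotDone gameplay tag from the player character.
; Two custom events teleport it to stored bank and vault locations and rotations.
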(event Custom|Teleport%20into%20bank
  (Transformation|Teleport (Variables|Default|GetBankTeleportLocation) (Variables|Default|GetBankTeleportRotation)))

(event Custom|Teleport%20into%20vault
  (Transformation|Teleport (Variables|Default|GetVaultTeleportLocation) (Variables|Default|GetVaultTeleportRotation)))

(event EventDialogueEvent
  (params (EventName :type Text))
  (switch string (Utilities|String|ToString(Text) EventName)
    (:VanLineDone
      (bind _asbp_main_character (Utilities|Casting|CastToBP_MainCharacter (Game|GetPlayerCharacter 0)))
      (GameplayTags|RemoveGameplayTag (Variables|/Game/Dynamic/Blueprints/Core/MC/BP_MainCharacter.BP_MainCharacter_C|GetOwnedGameplayTags _asbp_main_character) "(TagName=\"VanLineNotDone\")" :!class /Script/GameplayTags.BlueprintGameplayTagLibrary))))

(event EventInteract
  (Default|StartDialog (Variables|Default|GetBPC_DialogueComponent)))

(fn ConstructionScript)