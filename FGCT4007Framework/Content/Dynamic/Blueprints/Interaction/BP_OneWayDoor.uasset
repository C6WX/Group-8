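; BP_OneWayDoor is an interactable shop door that opens only once, then shuts automatically.
; Interact passes a DoOnce that is never reset and plays a timeline that swings the mesh's yaw open.
; Any overlap with DoorShut waits 1.5 seconds, then a second timeline swings it closed from a slightly wider angle than it opens to.
; The player pawn check on that overlap is left unconnected.
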(event OnComponentBeginOverlap(DoorShut)
  (params (OverlappedComponent :type Primitive%20Component%20Object%20Reference) (OtherActor :type Actor%20Object%20Reference) (OtherComp :type Primitive%20Component%20Object%20Reference) (OtherBodyIndex :type Integer) (bFromSweep :type Boolean) (SweepResult :type Hit%20Result%20Structure%20%28by%20ref%29))
  ;[1 1 1] Door shut automatically
  (Utilities|FlowControl|Delay 1.5)
  (bind _door_degree (Timeline|Door%20Degree Play)
    (:Update
      (Transformation|SetRelativeRotation (Variables|Default|GetSM_doorShop_02) (Math|Rotator|MakeRotator 0.0 0.0 (Math|Float|Lerp -1.1e+02 0.0 _door_degree)) false false))))

(event EventInteract
  ;[1 1 1] Open door once
  (Utilities|FlowControl|DoOnce false
    (:Completed
      (bind _doordegree (Timeline|DoorDegree Play)
        (:Update
          (Transformation|SetRelativeRotation (Variables|Default|GetSM_doorShop_02) (Math|Rotator|MakeRotator 0.0 0.0 (Math|Float|Lerp 0.0 -1e+02 _doordegree)) false false))))))

(fn ConstructionScript)