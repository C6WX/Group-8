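; BP_Cash is a cash pickup the player can steal, driven by a Pickup event.
; The event adds a fixed amount to the third-person character's Cash, prints the new total and destroys the actor.
; Gameplay tags on the character gate the theft: LeftEarly blocks it with a printed refusal unless ContinuedStealing is also present.
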(event Custom|Pickup
  (bind _asbp_third_person_character (Utilities|Casting|CastToBP_ThirdPersonCharacter (Game|GetPlayerCharacter 0)))
  (if (GameplayTags|HasTag (Variables|/Game/Dynamic/Blueprints/Core/MC/BP_ThirdPersonCharacter.BP_ThirdPersonCharacter_C|GetOwnedGameplayTags _asbp_third_person_character) "(TagName=\"ContinuedStealing\")")
    (bind _output_get (Variables|/Game/Dynamic/Blueprints/Core/MC/BP_ThirdPersonCharacter.BP_ThirdPersonCharacter_C|SetCash _asbp_third_person_character (+ (Variables|/Game/Dynamic/Blueprints/Core/MC/BP_ThirdPersonCharacter.BP_ThirdPersonCharacter_C|GetCash _asbp_third_person_character) 1e+03) :!label _label))
    (Development|PrintString (Utilities|String|ToString(Float) _output_get))
    (Actor|DestroyActor)
    (elif (GameplayTags|HasTag (Variables|/Game/Dynamic/Blueprints/Core/MC/BP_ThirdPersonCharacter.BP_ThirdPersonCharacter_C|GetOwnedGameplayTags _asbp_third_person_character) "(TagName=\"LeftEarly\")")
      (Development|PrintString "Can No Longer Steal")
      (else
        (goto _label)))))

(fn ConstructionScript)