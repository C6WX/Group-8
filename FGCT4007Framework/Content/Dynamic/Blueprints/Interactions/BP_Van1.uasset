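; BP_Van1 is an AI-driven van pawn with a scripted move to a hard-coded location.
; BeginPlay assigns its AI controller class, and a Test event runs AIMoveTo with that location and itself as goal actor.
; Tick looks up BP_VanTrigger every frame and feeds its TriggerVan flag into a DoOnce with nothing after it, so the trigger never starts the move.
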(event Custom|Test
  (bind _output_get (Variables|Default|SetMoveToLocation "-1994.232132,-3866.909007,35.503606"))
  (AI|AIMoveTo (AI|GetAIController 0) _output_get self -1.0 "Default" "Default" true true))

(event EventBeginPlay
  (Variables|Default|SetAIControllerClass "/Script/AIModule.AIController"))

(event Collision|EventActorBeginOverlap
  (params (OtherActor :type Actor%20Object%20Reference)))

(event EventTick
  (params (DeltaSeconds :type Float%20%28single-precision%29))
  (bind _returnvalue (Actor|GetActorOfClass "/Game/Dynamic/Blueprints/Interactions/BP_VanTrigger.BP_VanTrigger_C"))
  (if (Variables|/Game/Dynamic/Blueprints/Interactions/BP_VanTrigger.BP_VanTrigger_C|GetTriggerVan _returnvalue)
    (Utilities|FlowControl|DoOnce false)))

(event Input|KeyboardEvents|1
  (params (Key :type Key%20Structure :default "None")))

(fn ConstructionScript)