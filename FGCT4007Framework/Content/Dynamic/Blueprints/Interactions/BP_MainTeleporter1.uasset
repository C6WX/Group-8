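; BP_MainTeleporter1 is a one-shot trigger that teleports the player's BP_MainCharacter to a fixed location.
; Any overlap with its Box checks the player character's TP1Used flag and, if true, teleports the player and destroys the actor.
; An unconnected collapsed graph branches on bank-teller story outcome gameplay tags but never runs, and its repeated LeftKylieToKillTeller check leaves one exit unreachable.
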(event OnComponentBeginOverlap(Box)
  (params (OverlappedComponent :type Primitive%20Component%20Object%20Reference) (OtherActor :type Actor%20Object%20Reference) (OtherComp :type Primitive%20Component%20Object%20Reference) (OtherBodyIndex :type Integer) (bFromSweep :type Boolean) (SweepResult :type Hit%20Result%20Structure%20%28by%20ref%29))
  (bind _asbp_main_character (Utilities|Casting|CastToBP_MainCharacter (Game|GetPlayerCharacter 0)))
  (if (Variables|/Game/Dynamic/Blueprints/Core/MC/BP_MainCharacter.BP_MainCharacter_C|GetTP1%20Used _asbp_main_character)
    (Transformation|Teleport _asbp_main_character "-2231.000000,-2446.000000,-2393.000000" "0, 0, 0")
    (Actor|DestroyActor)))

(fn ConstructionScript)